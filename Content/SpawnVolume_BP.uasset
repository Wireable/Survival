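; SpawnVolume_BP is a spawn volume that provides a landscape ground check for candidate spawn locations.
; TraceLandscape casts a vertical object line trace against WorldStatic, spanning CollisionRange above and below the given location.
; It returns whether the hit actor is a Landscape, along with the impact point and normal.
; The event graph and construction script are empty, so the file shows no spawning logic or callers.
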(event EventBeginPlay)

(event EventActorBeginOverlap
  (params (OtherActor :type Actor%20Object%20Reference)))

(event EventTick
  (params (DeltaSeconds :type Float%20%28single-precision%29)))

(fn ConstructionScript)

(fn TraceLandscape
  (params (SpawnLocation :type Vector))
  (bind (_x _y _z) (Math|Vector|BreakVector SpawnLocation))
  (bind _collisionrange (Variables|Default|GetCollisionRange))
  (bind _outhit (Collision|LineTraceForObjects (Math|Vector|MakeVector _x _y (+ _z _collisionrange)) (Math|Vector|MakeVector _x _y (- _z _collisionrange)) (Utilities|Array|MakeArray (Utilities|Enum|LiteralenumEObjectTypeQuery "ObjectTypeQuery1")) false 0 "None"))
  (Utilities|Casting|CastToLandscape (.HitActor (Collision|BreakHitResult _outhit))
    (:then
      (LocalVariables|SethitLanscape true))
    (:CastFailed
      (LocalVariables|SethitLanscape false)))
  (return (LocalVariables|GethitLanscape) (.ImpactPoint (Collision|BreakHitResult _outhit)) (.ImpactNormal (Collision|BreakHitResult _outhit))))