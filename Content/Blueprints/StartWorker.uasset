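; StartWorker is a forest generator that divides a square around itself into grid cells and delegates tree placement to Worker actors.
; CallStarters runs once, randomly flagging unique cells for planting from a density-scaled tree count, then spawning the first Worker with the grid.
; It then messages all BPI_WorkerDispacher actors to start.
; Each finished Worker triggers the next from the last grid index, while reported tree counts accumulate for printing on completion.
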(event Custom|Destroy
  (Development|PrintString "DONE!")
  (Development|PrintString (Utilities|String|ToString(Integer) (Variables|Default|GetTotalTreesSpawned))))

(event Custom|CalcTrees
  (params (TreeNumber :type Integer))
  (Variables|Default|SetTotalTreesSpawned (+ TreeNumber (Variables|Default|GetTotalTreesSpawned))))

(event Custom|SpawnWorker
  (params (Index :type Integer))
  (Variables|Default|SetLastUsedGridIndex Index)
  (bind _returnvalue (Game|SpawnActorfromClass "/Game/Blueprints/Worker.Worker_C" (Math|Transform|MakeTransform "0, 0, 0") "AdjustIfPossibleButDontSpawnIfColliding" 0 (Variables|Control|GetTreeScaleMin) (Variables|Control|GetCollisionRangeTrace) (Variables|Control|GetMaxSlopeAngle) (Variables|Control|GetGridCellSize) (Variables|Control|GetMaxObjectsForWorker) (Variables|Default|GetLastUsedGridIndex) (Variables|Control|GetTreeRadius) (Variables|Control|GetActors%20To%20Spawn)))
  (Default|SetGridCellArray _returnvalue (Variables|Default|GetGrid))
  (EventDispatchers|BindEventtoFinishedWork _returnvalue (delegate Custom|SpawnWorker))
  (EventDispatchers|BindEventtoNumberOfTrees _returnvalue (delegate Custom|CalcTrees))
  (EventDispatchers|BindEventtoForestCreated _returnvalue (delegate Custom|Destroy)))

(event Custom|GenerateGrid
  (CallFunction|MaxTrees)
  (CallFunction|CreateGrid)
  (CallFunction|GenerateForest)
  (CallFunction|SpawnWorker (Variables|Default|GetLastUsedGridIndex)))

(event Custom|CallStarters
  (if (Variables|Default|GetWorkerActivated)
    (Variables|Default|SetWorkerActivated false)
    (CallFunction|GenerateGrid)
    (bind _outactors (Actor|GetAllActorswithInterface "/Game/Blueprints/BPI_WorkerDispacher.BPI_WorkerDispacher_C"))
    (Class|BPIWorkerDispacher|StartWorker(Message) _outactors)))

(fn ConstructionScript)

(fn MaxTrees
  (bind _radius (Variables|Control|GetRadius))
  (bind _gridcellsize (Variables|Control|GetGridCellSize))
  (bind _returnvalue (* _radius 2))
  (bind _returnvalue_2 (/ _returnvalue _gridcellsize))
  (Variables|Default|SetRows%20/%20Colums _returnvalue_2)
  (LocalVariables|SetTreeMax (Math|Float|Floor (Math|Float|Power (Math|Conversions|ToFloat(Integer) _returnvalue_2) 2.0)))
  (Variables|Control|SetTreeDensity (Math|Float|Clamp(Float) (Variables|Control|GetTreeDensity)))
  (Variables|Control|SetNumber%20of%20trees (Math|Float|Floor (* (Math|Integer|Clamp(Integer) (Variables|Control|GetNumber%20of%20trees) 0 (LocalVariables|GetTreeMax)) (Variables|Control|GetTreeDensity)))))

(fn CreateGrid
  (bind _returnvalue (Transformation|GetActorLocation))
  (bind _radius (Variables|Control|GetRadius))
  (bind _gridcellsize (Variables|Control|GetGridCellSize))
  (bind _rows___colums (Variables|Default|GetRows%20/%20Colums))
  (bind (_x _y _z) (Math|Vector|BreakVector _returnvalue))
  (bind _returnvalue_2 (- _rows___colums 1))
  (bind _returnvalue_3 (Math|Conversions|ToFloat(Integer) _radius))
  (bind _returnvalue_4 (/ _gridcellsize 2))
  (bind _returnvalue_5 (Math|Conversions|ToFloat(Integer) _returnvalue_4))
  (for _index (range 0 _returnvalue_2)
    (for _index_2 (range 0 _returnvalue_2)
      (bind _returnvalue_6 (Utilities|Array|Add (Variables|Default|GetGrid) (Utilities|Struct|MakeGridCell (Math|Vector|MakeVector (- (.X (Math|Vector|BreakVector (Math|Vector|MakeVector (- (+ _x _returnvalue_3) (Math|Conversions|ToFloat(Integer) (* _index _gridcellsize))) (- (+ _y _returnvalue_3) (Math|Conversions|ToFloat(Integer) (* _index_2 _gridcellsize))) _z))) _returnvalue_5) (- (.Y (Math|Vector|BreakVector (Math|Vector|MakeVector (- (+ _x _returnvalue_3) (Math|Conversions|ToFloat(Integer) (* _index _gridcellsize))) (- (+ _y _returnvalue_3) (Math|Conversions|ToFloat(Integer) (* _index_2 _gridcellsize))) _z))) _returnvalue_5) (.Z (Math|Vector|BreakVector (Math|Vector|MakeVector (- (+ _x _returnvalue_3) (Math|Conversions|ToFloat(Integer) (* _index _gridcellsize))) (- (+ _y _returnvalue_3) (Math|Conversions|ToFloat(Integer) (* _index_2 _gridcellsize))) _z)))) (Math|Vector|MakeVector (- (+ _x _returnvalue_3) (Math|Conversions|ToFloat(Integer) (* _index _gridcellsize))) (- (+ _y _returnvalue_3) (Math|Conversions|ToFloat(Integer) (* _index_2 _gridcellsize))) _z) (Math|Vector|MakeVector (- (.X (Math|Vector|BreakVector (Math|Vector|MakeVector (- (.X (Math|Vector|BreakVector (Math|Vector|MakeVector (- (+ _x _returnvalue_3) (Math|Conversions|ToFloat(Integer) (* _index _gridcellsize))) (- (+ _y _returnvalue_3) (Math|Conversions|ToFloat(Integer) (* _index_2 _gridcellsize))) _z))) _returnvalue_5) (- (.Y (Math|Vector|BreakVector (Math|Vector|MakeVector (- (+ _x _returnvalue_3) (Math|Conversions|ToFloat(Integer) (* _index _gridcellsize))) (- (+ _y _returnvalue_3) (Math|Conversions|ToFloat(Integer) (* _index_2 _gridcellsize))) _z))) _returnvalue_5) (.Z (Math|Vector|BreakVector (Math|Vector|MakeVector (- (+ _x _returnvalue_3) (Math|Conversions|ToFloat(Integer) (* _index _gridcellsize))) (- (+ _y _returnvalue_3) (Math|Conversions|ToFloat(Integer) (* _index_2 _gridcellsize))) _z)))))) _returnvalue_5) (- (.Y (Math|Vector|BreakVector (Math|Vector|MakeVector (- (.X (Math|Vector|BreakVector (Math|Vector|MakeVector (- (+ _x _returnvalue_3) (Math|Conversions|ToFloat(Integer) (* _index _gridcellsize))) (- (+ _y _returnvalue_3) (Math|Conversions|ToFloat(Integer) (* _index_2 _gridcellsize))) _z))) _returnvalue_5) (- (.Y (Math|Vector|BreakVector (Math|Vector|MakeVector (- (+ _x _returnvalue_3) (Math|Conversions|ToFloat(Integer) (* _index _gridcellsize))) (- (+ _y _returnvalue_3) (Math|Conversions|ToFloat(Integer) (* _index_2 _gridcellsize))) _z))) _returnvalue_5) (.Z (Math|Vector|BreakVector (Math|Vector|MakeVector (- (+ _x _returnvalue_3) (Math|Conversions|ToFloat(Integer) (* _index _gridcellsize))) (- (+ _y _returnvalue_3) (Math|Conversions|ToFloat(Integer) (* _index_2 _gridcellsize))) _z)))))) _returnvalue_5) (.Z (Math|Vector|BreakVector (Math|Vector|MakeVector (- (.X (Math|Vector|BreakVector (Math|Vector|MakeVector (- (+ _x _returnvalue_3) (Math|Conversions|ToFloat(Integer) (* _index _gridcellsize))) (- (+ _y _returnvalue_3) (Math|Conversions|ToFloat(Integer) (* _index_2 _gridcellsize))) _z))) _returnvalue_5) (- (.Y (Math|Vector|BreakVector (Math|Vector|MakeVector (- (+ _x _returnvalue_3) (Math|Conversions|ToFloat(Integer) (* _index _gridcellsize))) (- (+ _y _returnvalue_3) (Math|Conversions|ToFloat(Integer) (* _index_2 _gridcellsize))) _z))) _returnvalue_5) (.Z (Math|Vector|BreakVector (Math|Vector|MakeVector (- (+ _x _returnvalue_3) (Math|Conversions|ToFloat(Integer) (* _index _gridcellsize))) (- (+ _y _returnvalue_3) (Math|Conversions|ToFloat(Integer) (* _index_2 _gridcellsize))) _z))))))) false)))
      (Utilities|Array|Add (Variables|Default|GetRandGrid) _returnvalue_6))))

(fn GenerateForest
  (bind _grid (Variables|Default|GetGrid))
  (for _index (range 0 (- (Variables|Control|GetNumber%20of%20trees) 1))
    (LocalVariables|SetRandom%20Index (Math|Random|RandomIntegerinRange 0 (Utilities|Array|LastIndex (Variables|Default|GetRandGrid))))
    (LocalVariables|SetRandomCell (Utilities|Array|Get(acopy) _grid (Utilities|Array|Get(acopy) (Variables|Default|GetRandGrid) (LocalVariables|GetRandom%20Index))))
    (Utilities|Array|SetArrayElem _grid (Utilities|Array|Get(acopy) (Variables|Default|GetRandGrid) (LocalVariables|GetRandom%20Index)) (Utilities|Struct|MakeGridCell (.Center_2 (Utilities|Struct|BreakGridCell (LocalVariables|GetRandomCell))) (.TopLeft_5 (Utilities|Struct|BreakGridCell (LocalVariables|GetRandomCell))) (.BottomRight_8 (Utilities|Struct|BreakGridCell (LocalVariables|GetRandomCell))) true))
    (Utilities|Array|RemoveIndex (Variables|Default|GetRandGrid) (LocalVariables|GetRandom%20Index))))