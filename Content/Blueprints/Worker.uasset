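; Short-lived worker actor that spawns one batch of random trees on grid cells flagged for planting, as part of forest generation.
; Each tree gets a jittered position, line trace onto Landscape, slope check, random yaw and scale, and is sunk by slope and radius.
; It stops past an object budget counting cells and trees, reports tree count plus resume index or forest completion through dispatchers, then destroys itself.
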(event Custom|Break%20loop
  (Utilities|FlowControl|ForLoopwithBreak (Variables|Default|GetLastUsedGridIndex) (Utilities|Array|LastIndex (Variables|Default|GetGrid))) ; enters at Break
)

(event EventStartWorker
  (if (Variables|Default|GetbStartWork)
    (Variables|Default|SetbStartWork false)
    (Variables|Default|SetLastUsedGridIndex (+ (Variables|Default|GetLastUsedGridIndex) 1))
    (bind _index (Utilities|FlowControl|ForLoopwithBreak (Variables|Default|GetLastUsedGridIndex) (Utilities|Array|LastIndex (Variables|Default|GetGrid)))
      (:LoopBody
        (Variables|Default|SetGridCell (Utilities|Array|Get(acopy) (Variables|Default|GetGrid) _index))
        (Utilities|FlowControl|Sequence
          (:then_0
            (if (.bPlantTree_10 (Utilities|Struct|BreakGridCell (Variables|Default|GetGridCell)))
              (CallFunction|AddTrees (Variables|Default|GetGridCell))))
          (:then_1
            (Variables|Default|SetLastUsedGridIndex _index)
            (Variables|Default|SetCreatedObjects (+ 1 (Variables|Default|GetCreatedObjects)))
            (if (> (Variables|Default|GetCreatedObjects) (Variables|Default|GetMaxObjectsToCreate))
              (Variables|Default|SetbSpawn true)
              (CallFunction|BreakLoop)))))
      (:Completed
        (Default|CallNumberOfTrees (Variables|Default|GetTreesSpawnedCount) :!label _label)
        (if (Variables|Default|GetbSpawn)
          (Default|CallFinishedWork (Variables|Default|GetLastUsedGridIndex))
          (else
            (Default|CallForestCreated)))
        (Actor|DestroyActor)))
    (else
      (goto _label))))

(fn ConstructionScript)

(fn AddTrees
  (params (Cell :type Grid%20Cell%20Structure))
  (bind _center_2 (Utilities|Struct|BreakGridCell Cell))
  (bind _treeactors (Variables|Default|GetTreeActors))
  (bind _treescalemin (Variables|Default|GetTreeScaleMin))
  (bind (_x _y _z) (Math|Vector|BreakVector _center_2))
  (bind _returnvalue (Math|Random|RandomFloatinRange _treescalemin 1.0))
  (LocalVariables|SetRandIdx (Math|Random|RandomIntegerinRange 0 (Utilities|Array|LastIndex _treeactors)))
  (Variables|Default|SetRandom%20Tree%20Actor (Utilities|Array|Get(acopy) _treeactors (LocalVariables|GetRandIdx)))
  (LocalVariables|SetTreeRadius (Utilities|Array|Get(acopy) (Variables|Default|GetTreeRadiusArray) (LocalVariables|GetRandIdx)))
  (LocalVariables|SetSafeDistance (Math|Conversions|ToFloat(Integer) (/ (- (Variables|Default|GetGridCellSize) (Math|Float|Floor (LocalVariables|GetTreeRadius))) 2)))
  (LocalVariables|SetTreeSpawnPosition (Math|Vector|MakeVector (+ _x (Math|Random|RandomFloatinRange (* (LocalVariables|GetSafeDistance) -1.0) (LocalVariables|GetSafeDistance))) (+ _y (Math|Random|RandomFloatinRange (* (LocalVariables|GetSafeDistance) -1.0) (LocalVariables|GetSafeDistance))) _z))
  (bind (_hitresult _bhit) (CallFunction|Trace (LocalVariables|GetTreeSpawnPosition)))
  (if _bhit
    (bind (_slopeangle _bcanspawn) (CallFunction|CheckSlopeAngle (LocalVariables|GetTreeSpawnPosition) _hitresult))
    (LocalVariables|SetSlopeAngle _slopeangle)
    (if _bcanspawn
      (LocalVariables|SetTraceHitLocation (.Location (Collision|BreakHitResult _hitresult)))
      (Game|SpawnActorfromClass (Variables|Default|GetRandom%20Tree%20Actor) (Math|Transform|MakeTransform (Math|Vector|MakeVector (.X (Math|Vector|BreakVector (LocalVariables|GetTraceHitLocation))) (.Y (Math|Vector|BreakVector (LocalVariables|GetTraceHitLocation))) (- (.Z (Math|Vector|BreakVector (LocalVariables|GetTraceHitLocation))) (* (Math|Trig|Tan(Degrees) (LocalVariables|GetSlopeAngle)) (LocalVariables|GetTreeRadius)))) (Math|Rotator|MakeRotator 0.0 0.0 (Math|Random|RandomFloatinRange 0.0 3.6e+02)) (Math|Vector|MakeVector _returnvalue _returnvalue _returnvalue)) "Undefined" 0 0)
      (Variables|Default|SetCreatedObjects (+ (Variables|Default|GetCreatedObjects) 1))
      (Variables|Default|SetTreesSpawnedCount (+ (Variables|Default|GetTreesSpawnedCount) 1)))))

(fn CheckSlopeAngle
  (params (ToSpawnPosition :type Vector) (TraceHit :type Hit%20Result%20Structure))
  (bind (_bblockinghit _binitialoverlap _time _location _impactpoint _normal _impactnormal) (Collision|BreakHitResult TraceHit))
  (bind (_x _y _z) (Math|Vector|BreakVector ToSpawnPosition))
  (bind _collisionrangetrace (Variables|Default|GetCollisionRangeTrace))
  (bind _returnvalue (+ _z _collisionrangetrace))
  (bind _returnvalue_2 (Math|Vector|MakeVector _x _y _returnvalue))
  (bind _returnvalue_3 (- _returnvalue_2 _impactpoint))
  (bind _returnvalue_4 (Math|Vector|Normalize _returnvalue_3))
  (LocalVariables|SetAngle (Class|KismetMathLibrary|DegAcos (/ (Math|Vector|DotProduct _returnvalue_4 _impactnormal) (* (Math|Vector|VectorLength _returnvalue_4) (Math|Vector|VectorLength _impactnormal)))))
  (return (LocalVariables|GetAngle) (and (<= (LocalVariables|GetAngle) (Variables|Default|GetMaxSlopeAngle)) (>= (LocalVariables|GetAngle) 0.0))))

(fn Trace
  (params (SpawnToTrace :type Vector))
  (bind (_x _y _z) (Math|Vector|BreakVector SpawnToTrace))
  (bind _collisionrangetrace (Variables|Default|GetCollisionRangeTrace))
  (bind _outhit (Collision|LineTraceForObjects (Math|Vector|MakeVector _x _y (+ _z _collisionrangetrace)) (Math|Vector|MakeVector _x _y (- _z _collisionrangetrace)) (Utilities|Array|MakeArray "ObjectTypeQuery1") true 0 "None"))
  (Utilities|Casting|CastToLandscape (.HitActor (Collision|BreakHitResult _outhit))
    (:then
      (LocalVariables|SetLandscapeHit true))
    (:CastFailed
      (LocalVariables|SetLandscapeHit false)))
  (return _outhit (LocalVariables|GetLandscapeHit)))

(fn SetGridCellArray
  (params (GridCellArray :type Array%20of%20Grid%20Cell%20Structures))
  (Variables|Default|SetGrid GridCellArray))