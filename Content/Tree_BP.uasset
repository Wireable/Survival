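; Tree actor that takes damage and topples as a physics object once its health runs out.
; AnyDamage subtracts damage from Health and prints the remaining value to screen.
; At zero or below, it casts the first child of the default scene root to a static mesh component and enables physics simulation on it.
; The construction script only calls its parent.
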(event EventBeginPlay)

(event EventActorBeginOverlap
  (params (OtherActor :type Actor%20Object%20Reference)))

(event EventTick
  (params (DeltaSeconds :type Float%20%28single-precision%29)))

(event Game|Damage|EventAnyDamage
  (params (Damage :type Float%20%28single-precision%29) (DamageType :type Damage%20Type%20Object%20Reference) (InstigatedBy :type Controller%20Object%20Reference) (DamageCauser :type Actor%20Object%20Reference))
  (bind _output_get (Variables|Default|SetHealth (- (Variables|Default|GetHealth) Damage)))
  (Development|PrintString (Utilities|String|ToString(Float) _output_get))
  (if (<= _output_get 0.0)
    (bind _asstatic_mesh_component (Utilities|Casting|CastToStaticMeshComponent (Components|GetChildComponent (Variables|Default|GetDefaultSceneRoot) 0)))
    (Physics|SetSimulatePhysics _asstatic_mesh_component true)))

(fn ConstructionScript
  (|CallParentFunction))